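; Medkit is a usable pickup item that heals the first-person character who uses it.
; Its Use event casts the owner to FP_char, adds a fixed amount to Health clamped to the valid range, then destroys the item.
; The construction script only calls its parent, and the default events are disabled.
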(event `/Game/Interactable_objects/Iteract_interface.Use`
  (params (Owner :type "Actor Object Reference"))
  (bind _asfp_char (cast `/Game/FP/CharBP/FP_char` Owner))
  (set `/Game/FP/CharBP/FP_char.Health` (`KismetMathLibrary.FClamp` (+ (`/Game/FP/CharBP/FP_char.Health` _asfp_char) 50.0) 0.0 100.0) _asfp_char)
  (`self.K2_DestroyActor`))

(event `self.ReceiveBeginPlay`)

(event `self.ReceiveActorBeginOverlap`
  (params (OtherActor :type "Actor Object Reference")))

(event `self.ReceiveTick`
  (params (DeltaSeconds :type "Float (single-precision)")))

(fn `UserConstructionScript`
  (`parent.UserConstructionScript`))