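; Binocular device that reuses the parent weapon's fire action to set a narrower aim zoom instead of shooting.
; ShootGun prints a debug string, then sets its AimZoom and the player FP_char's WeaponAimZoom to a fraction of the current follow camera FOV.
; The construction script extends the parent's, adding one fire mode and zeroing aim recoil and initial zoom.
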(event `/Game/Weapons/Weapon_interface.ShootGun`
  (`KismetSystemLibrary.PrintString` "Hello")
  (bind _asfp_char (cast `/Game/FP/CharBP/FP_char` (`GameplayStatics.GetPlayerCharacter` 0)))
  (bind _returnvalue (* (`CameraComponent.FieldOfView` (`/Game/FP/CharBP/FP_char.FollowCamera` _asfp_char)) 0.875))
  (set `self.AimZoom` _returnvalue)
  (set `/Game/FP/CharBP/FP_char.WeaponAimZoom` _returnvalue _asfp_char))

(event `self.ReceiveActorBeginOverlap`
  (params (OtherActor :type "Actor Object Reference")))

(event `self.ReceiveTick`
  (params (DeltaSeconds :type "Float (single-precision)")))

(fn `UserConstructionScript`
  (`parent.UserConstructionScript`)
  (`KismetArrayLibrary.Array_Add` (`self.FireMode`) "NewEnumerator0")
  (set `self.AimRecoilScale` 0.0)
  (set `self.AimZoom` 0.0))