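; M1911 pistol Blueprint, a data-only style child of a parent weapon class that defines this gun's handling.
; The construction script calls the parent's, then overrides fire rate and mode, reload time, aim and hip positions, weapon and hand rotations, and the hands animation class.
; It assigns the 7.62 bullet type despite the M1911 name.
; The event graph holds only disabled stub events, so runtime logic is not defined here.
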(event `self.ReceiveBeginPlay`)

(event `self.ReceiveActorBeginOverlap`
  (params (OtherActor :type "Actor Object Reference")))

(event `self.ReceiveTick`
  (params (DeltaSeconds :type "Float (single-precision)")))

(fn `UserConstructionScript`
  (`parent.UserConstructionScript`)
  (set `self.FireRate` 0.5)
  (set `self.AimPosition` (-29.927006 -1.070973 -10.381394))
  (set `self.NoAimPosition` (-20.964308 20.070066 -22.209999))
  (set `self.BS_Default` (`|MakeArray` 1.0 -1.0 1.0 -1.0 :!type "Float (single-precision)"))
  (set `self.ReloadTime` 3.8)
  (set `self.FireMode` "NewEnumerator1")
  (set `self.BulletType` "/Game/Weapons/Bullet/7_62/7_62_Bullet.7_62_Bullet_C")
  (set `self.WeaponRotationinHands` (struct :`Pitch` 4.5 :`Yaw` -14.3 :`Roll` 1.5))
  (set `self.HandsRotation` (struct :`Yaw` 89.32093))
  (set `self.HandsAnimClass` "/Game/Weapons/Auto_weapon/m1911/AnimBP/m1911Hands_AB.m1911Hands_AB_C"))