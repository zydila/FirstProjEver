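; AK automatic rifle Blueprint that configures a parent weapon class for this specific gun.
; The construction script runs the parent's, then sets fire rate and mode, aim and hip positions, reload time, 7.62 bullet type, hands rotation and anim class, and the muzzle flash particle.
; IncreaseRecoil and DecreaseRecoil play and reverse one timeline, whose update drives RecoilScale so recoil ramps up and back down.
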(event `self.IncreaseRecoil`
  (bind (_direction _newtrack_3) (`Timeline|Timeline_0` :!label _label)
    (:`Update`
      (set `self.RecoilScale` _newtrack_3))))

(event `self.DecreaseRecoil`
  (goto _label :!via `Reverse`))

(event `self.ReceiveBeginPlay`)

(event `self.ReceiveActorBeginOverlap`
  (params (OtherActor :type "Actor Object Reference")))

(event `self.ReceiveTick`
  (params (DeltaSeconds :type "Float (single-precision)")))

(fn `UserConstructionScript`
  (`parent.UserConstructionScript`)
  (set `self.FireRate` 0.1)
  (set `self.AimPosition` (-11.725622 -11.929688 -11.626453))
  (set `self.NoAimPosition` (-11.725611 -0.228236 -20.045261))
  (set `self.BS_Default` (`|MakeArray` 1.0 -1.0 1.0 -1.0 :!type "Float (single-precision)"))
  (set `self.ReloadTime` 3.8)
  (set `self.FireMode` "NewEnumerator1")
  (set `self.BulletType` "/Game/Weapons/Bullet/7_62/7_62_Bullet.7_62_Bullet_C")
  (set `self.HandsRotation` (struct :`Yaw` 90.0))
  (set `self.WeaponRotationinHands` (struct))
  (set `self.HandsAnimClass` "/Game/Weapons/Auto_weapon/AK/AnimBP/akHands_AB.akHands_AB_C")
  (`ParticleSystemComponent.SetTemplate` (`self.Flash`) "/Game/StarterContent/Particles/P_Sparks.P_Sparks"))